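; NPC character Blueprint that toggles a dialogue indicator around interactions.
; It overrides the inherited StartInteraction and EndInteraction, calling the parent logic, then hiding DialogueIndicator on start and showing it again on end.
; The construction script only calls its parent, and the Tick event is empty, with its parent call left unconnected.
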(event `self.ReceiveTick`
  (params (DeltaSeconds :type "Float (single-precision)")))

(fn `EndInteraction`
  (`parent.EndInteraction`)
  (`SceneComponent.SetVisibility` (`self.DialogueIndicator`) true false))

(fn `StartInteraction`
  (`parent.StartInteraction`)
  (`SceneComponent.SetVisibility` (`self.DialogueIndicator`) false false))

(fn `UserConstructionScript`
  (`parent.UserConstructionScript`))