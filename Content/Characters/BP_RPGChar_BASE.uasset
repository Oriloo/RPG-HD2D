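; Base Blueprint for RPG characters that handles dialogue interactions between them.
; On BeginPlay it adds the start menu widget to the viewport and caches the gameplay game mode.
; Interact puts both instigator and self into interaction, setting a lock flag and halting movement, then opens dialogue through the game mode's HUD widget and prints a placeholder line.
; FinishInteraction clears the lock on this character only.
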(event `self.ReceiveBeginPlay`
  (bind _returnvalue (`|CreateWidget` "/Game/Widgets/WBP_StartMenu.WBP_StartMenu_C" (`GameplayStatics.GetPlayerController` 0)))
  (`UserWidget.AddToViewport` _returnvalue 0)
  (bind _asgm_gameplay (cast `/Game/Blueprints/GM_Gameplay` (`GameplayStatics.GetGameMode`)))
  (set `self.GameMode` _asgm_gameplay))

(event `self.ReceiveActorBeginOverlap`
  (params (OtherActor :type "Actor Object Reference"))
  (`parent.ReceiveActorBeginOverlap` OtherActor))

(event `/Game/Characters/Interfaces/BPI_Interaction.Interact`
  (params (Instigator :type "/Game/Characters/BP_RPGChar_BASE Object Reference"))
  (`self.StartInteraction` Instigator)
  (`self.StartInteraction`)
  (bind _dialogue (`self.ShowDialogueLine`))
  (`KismetSystemLibrary.PrintString` _dialogue))

(event `/Game/Characters/Interfaces/BPI_Interaction.FinishInteraction`
  (`self.EndInteraction`))

(fn `EndInteraction`
  (set `self.isInteractionLocked` false))

(fn `ShowDialogueLine`
  (returns (Dialogue :type String))
  (`/Game/Widgets/WBP_HUD.ShowDialogue` (`/Game/Blueprints/GM_Gameplay.HUDWidget` (`self.GameMode`)) self)
  (return "Hello BP !"))

(fn `StartInteraction`
  (set `self.isInteractionLocked` true)
  (`MovementComponent.StopMovementImmediately` (`self.CharacterMovement`)))

(fn `UserConstructionScript`)