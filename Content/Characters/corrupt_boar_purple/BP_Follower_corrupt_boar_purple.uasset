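; Blueprint for the purple corrupt boar follower, a turn-based combat character.
; On BeginPlay it fills four attack data components with elemental, physical and spirit damage actions, the fourth pairing elemental damage with a timed heal.
; Each tick, while the turn combat component reports its turn, it tells the combat policy runner to execute an action.
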(event `self.ReceiveTick`
  (params (DeltaSeconds :type "Float (single-precision)"))
  (if (`UTurnCombatComponent.bIsMyTurn` (`self.UTurnCombat`))
    (`CombatPolicyRunner.executeAction` (`self.CombatPolicyRunner`))))

(event `self.ReceiveBeginPlay`
  (`UAttackDataComponent.addAction` (`self.UAttackData`) "elm" 10 0)
  (`UAttackDataComponent.addAction` (`self.UAttackData1`) "phy" 10 0)
  (`UAttackDataComponent.addAction` (`self.UAttackData2`) "spr" 10 0)
  (`UAttackDataComponent.addAction` (`self.UAttackData3`) "elm" 10 0)
  (`UAttackDataComponent.addAction` (`self.UAttackData3`) "Heal" 10 2))

(fn `UserConstructionScript`
  (`parent.UserConstructionScript`))