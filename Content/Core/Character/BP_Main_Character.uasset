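; Main character Blueprint that handles axis-driven movement and sets up its attack data at startup.
; The MoveRight axis moves it along the forward vector constant and MoveForward along the actor's right vector, so the axis names are crossed relative to their directions.
; On BeginPlay it adds actions to four attack data objects with elemental, physical and "spr" types, the last pairing elemental damage with a timed Heal.
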(event `InputAxis|MoveRight`
  (params (AxisValue :type "Float (single-precision)"))
  (`self.AddMovementInput` (`KismetMathLibrary.Vector_Forward`) AxisValue))

(event `InputAxis|MoveForward`
  (params (AxisValue :type "Float (single-precision)"))
  (`self.AddMovementInput` (`self.GetActorRightVector`) AxisValue))

(event `self.ReceiveBeginPlay`
  (`UAttackDataComponent.addAction` (`self.UAttackData`) "elm" 10 0)
  (`UAttackDataComponent.addAction` (`self.UAttackData1`) "phy" 10 0)
  (`UAttackDataComponent.addAction` (`self.UAttackData2`) "spr" 10 0)
  (`UAttackDataComponent.addAction` (`self.UAttackData3`) "elm" 10 0)
  (`UAttackDataComponent.addAction` (`self.UAttackData3`) "Heal" 10 2))

(fn `UserConstructionScript`)